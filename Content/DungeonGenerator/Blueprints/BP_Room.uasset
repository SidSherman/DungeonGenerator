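; BP_Room is a procedural dungeon room that builds a tiled rectangle with walls and doors in its construction script.
; BuildRoom fills an instanced floor grid, then walks the four edges, marking every DoorEvery-th tile, offset by DoorRemainder, as a door candidate.
; WallOrDoorSelector rolls candidates on a random stream, weighted by DoorCount and doors already placed, to spawn a BP_Door actor, otherwise adding a wall instance.
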(event EventBeginPlay)

(event Collision|EventActorBeginOverlap
  (params (OtherActor :type Actor%20Object%20Reference)))

(event EventTick
  (params (DeltaSeconds :type Float%20%28single-precision%29)))

(fn ConstructionScript
  (CallFunction|BuildRoom))

(fn BuildRoom
  (bind _doorevery (Variables|Default|GetDoorEvery))
  (bind _doorevery_2 (Variables|Default|GetDoorEvery))
  ;[1 1 1] Floors
  ;;[1 1 1] Rows
  (for _index (range 0 (- (Variables|RoomSize|GetRoomTileY) 1))
    ;;[1 1 1] Columns
    (for _index_2 (range 0 (- (Variables|RoomSize|GetRoomTileX) 1))
      (Components|InstancedStaticMesh|AddInstance (Variables|Default|GetFloor) (Math|Transform|MakeTransform (Math|Vector|MakeVector (* _index_2 (Variables|RoomSize|GetTileSizeX)) (* _index (Variables|RoomSize|GetTileSizeY)) 0.0) "0, 0, 0" "1.000000,1.000000,1.000000") false)))
  ;[1 1 1] Walls
  ;;[1 1 1] Bottom
  (for _index_3 (range 0 (- (Variables|RoomSize|GetRoomTileY) 1))
    (CallFunction|WallorDoorSelector (Math|Vector|MakeVector 0.0 (* _index_3 (Variables|RoomSize|GetTileSizeY)) 0.0) "0.000000,90.000000,0.000000" (== (Math|Integer|%(Integer) _index_3 _doorevery) (Math|Integer|Clamp(Integer) (Variables|Default|GetDoorRemainder) 0 (- _doorevery 1))))
    ;;[1 1 1] Top
    (CallFunction|WallorDoorSelector (Math|Vector|MakeVector (* (Variables|RoomSize|GetRoomTileX) (Variables|RoomSize|GetTileSizeX)) (* (+ _index_3 1) (Variables|RoomSize|GetTileSizeY)) 0.0) "0.000000,-90.000000,0.000000" (== (Math|Integer|%(Integer) _index_3 _doorevery) (Math|Integer|Clamp(Integer) (Variables|Default|GetDoorRemainder) 0 (- _doorevery 1)))))
  ;;[1 1 1] left
  (for _index_4 (range 0 (- (Variables|RoomSize|GetRoomTileX) 1))
    (CallFunction|WallorDoorSelector (Math|Vector|MakeVector (* (Variables|RoomSize|GetTileSizeX) _index_4) (* (Variables|RoomSize|GetRoomTileY) (Variables|RoomSize|GetTileSizeY)) 0.0) "0, 0, 0" (== (Math|Integer|%(Integer) _index_4 _doorevery_2) (Math|Integer|Clamp(Integer) (Variables|Default|GetDoorRemainder) 0 (- _doorevery_2 1))))
    ;;[1 1 1] Right
    (CallFunction|WallorDoorSelector (Math|Vector|MakeVector (* (+ _index_4 1) (Variables|RoomSize|GetTileSizeX)) 0.0 0.0) "0.000000,180.000000,0.000000" (== (Math|Integer|%(Integer) _index_4 _doorevery_2) (Math|Integer|Clamp(Integer) (Variables|Default|GetDoorRemainder) 0 (- _doorevery_2 1))))))

(fn WallorDoorSelector
  (params (Instance%20Transform%20Location :type Vector) (Instance%20Transform%20Rotation :type Rotator) (bCanDoor :type Boolean))
  (bind _returnvalue (Transformation|GetActorTransform))
  (bind _doorcount (Variables|Default|GetDoorCount))
  ;[1 1 1] Spawn Door
  (if (and bCanDoor (Class|KismetMathLibrary|RandomBoolwithWeightfromStream (/ _doorcount (Math|Conversions|ToFloat(Integer) (- _doorcount (Utilities|Array|Length (Variables|Default|GetDoors))))) (Variables|Default|GetRandom%20Stream)))
    (bind _returnvalue_2 (Game|SpawnActorfromClass "/Game/StarterContent/Architecture/BP_Door.BP_Door_C" (Math|Transform|MakeTransform (Math|Transform|TransformLocation _returnvalue Instance%20Transform%20Location) (Math|Transform|TransformRotation _returnvalue Instance%20Transform%20Rotation) "1.000000,1.000000,1.000000") "Undefined" 0 0))
    (Utilities|Array|Add (Variables|Default|GetDoors) _returnvalue_2)
    (else
      ;[1 1 1] Spawn Wall
      (Components|InstancedStaticMesh|AddInstance (Variables|Default|GetWall) (Math|Transform|MakeTransform Instance%20Transform%20Location Instance%20Transform%20Rotation "1.000000,1.000000,1.000000") false))))